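; BP_FPSGameMode is the FPS game mode that handles player respawn and the pause menu.
; On BeginPlay it binds to an OnPlayerDied event and restarts the dead character's controller through RestartPlayer.
; PauseGame lazily creates a cached WBP_Pause widget, then toggles pause, adding or removing the menu and switching mouse cursor and input mode for player 0.
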(event `self.ReceiveBeginPlay`
  (add `self.OnPlayerDied` (delegate `PlayerDied`)))

(event `PlayerDied` :!signature `self.OnPlayerDied`
  (params (Character :type "/Game/Source/Character/BP_Character Object Reference"))
  (`self.RestartPlayer` (`Pawn.GetController` Character)))

(event `PauseGame`
  (bind _returnvalue (`GameplayStatics.GetPlayerController` 0))
  (`/Engine/EditorBlueprintResources/StandardMacros.IsValid` (`self.PauseMenu`)
    (:`Is Valid`
      _)
    (:`Is Not Valid`
      (bind _returnvalue_2 (`|CreateWidget` "/Game/Source/WBP/WBP_Pause.WBP_Pause_C"))
      (bind _output_get (set `self.PauseMenu` _returnvalue_2))))
  (if (`GameplayStatics.IsGamePaused`)
    (`Widget.RemoveFromParent` _output_get)
    (`GameplayStatics.SetGamePaused` false)
    (set `PlayerController.bShowMouseCursor` false _returnvalue)
    (`WidgetBlueprintLibrary.SetInputMode_GameOnly` _returnvalue)
    (else
      (`UserWidget.AddToViewport` _output_get 0)
      (`GameplayStatics.SetGamePaused` true)
      (set `PlayerController.bShowMouseCursor` true _returnvalue)
      (`WidgetBlueprintLibrary.SetInputMode_GameAndUIEx` _returnvalue null "LockInFullscreen" false))))

(fn `UserConstructionScript`)