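; First-person player controller that handles input setup, the interaction HUD and the death-and-restart sequence.
; BeginPlay adds the character Enhanced Input mapping context, and possessing a BP_Character creates the interact widget.
; OnDeath fades the camera out and shows a timed death widget, then calls the character's restart, re-possesses it and stops the fade.
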(event `self.ReceiveBeginPlay`
  (`EnhancedInputSubsystemInterface.AddMappingContext` (subsystem `EnhancedInputLocalPlayerSubsystem`) "/Game/Source/Input/IM_Character.IM_Character" 0 (struct)))

(event `self.ReceivePossess`
  (params (PossessedPawn :type "Pawn Object Reference"))
  (cast `/Game/Source/Character/BP_Character` PossessedPawn)
  (bind _returnvalue (`|CreateWidget` "/Game/Source/WBP/WBP_Interact.WBP_Interact_C" self))
  (bind _output_get (set `self.Interact Widget` _returnvalue))
  (`UserWidget.AddToViewport` _output_get 0))

(event `OnDeath`
  (bind _returnvalue (`GameplayStatics.GetPlayerCharacter` 0))
  (bind _playercameramanager (`self.PlayerCameraManager`))
  (`PlayerCameraManager.StartCameraFade` :`self` _playercameramanager :`ToAlpha` 1.0 :`Duration` 1.0 :`bHoldWhenFinished` true)
  (bind _returnvalue_2 (`|CreateWidget` "/Game/Source/WBP/WBP_PlayerDie.WBP_PlayerDie_C"))
  (`UserWidget.AddToViewport` _returnvalue_2 0)
  (`KismetSystemLibrary.Delay` 3.0)
  (`Widget.RemoveFromParent` _returnvalue_2)
  (`KismetSystemLibrary.Delay` 0.2)
  (bind _asbp_character (cast `/Game/Source/Character/BP_Character` _returnvalue))
  (`/Game/Source/Character/BP_Character.CallRestart` _asbp_character)
  (`self.Possess` _returnvalue)
  (`PlayerCameraManager.StopCameraFade` _playercameramanager))

(fn `UserConstructionScript`)