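; First-person player character handling movement, look, jump, run, pause requests and health, notifying the player controller on death.
; Each tick, a camera line trace shows the interact widget and sets CanInteract when it hits a BI_Interact actor.
; Interact input sends lever, button and glasses interface messages to that actor.
; Glasses functions switch color vision deficiency simulation between tritanope and normal, though both set GlassesOn to true.
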(event `self.ReceiveBeginPlay`
  ;[0 1 0.2247] Begin Play
  (bind _returnvalue (`|CreateWidget` "/Game/Source/UMG/WB_Interact.WB_Interact_C")) ; ajout du widget d'interaction
  (set `self.Interact_Widget` _returnvalue))

(event `self.ReceiveTick`
  (params (DeltaSeconds :type "Float (single-precision)"))
  (bind _firstpersoncamera (`self.FirstPersonCamera`))
  (bind _interact_widget (`self.Interact_Widget`))
  (bind _returnvalue (`SceneComponent.K2_GetComponentLocation` _firstpersoncamera))
  (bind _returnvalue_2 (`Widget.IsInViewport` (`self.Interact_Widget`)))
  ;[1 0 0] Interaction
  (`self.Interact_Widget`
    (:`then`
      (bind (_outhit _returnvalue_3) (`KismetSystemLibrary.LineTraceSingle` _returnvalue (+ _returnvalue (* (`SceneComponent.GetForwardVector` _firstpersoncamera) 500.0)) "TraceTypeQuery1")) ; Raycast
      (if _returnvalue_3
        (if (`KismetSystemLibrary.DoesImplementInterface` (`.HitActor` (`GameplayStatics.BreakHitResult` _outhit)) "/Game/Source/Blueprints/Interfaces/BI_Interact.BI_Interact_C")
          (if (not _returnvalue_2)
            (`UserWidget.AddToViewport` _interact_widget 0)
            (set `self.Can_Interact` true))
          (else
            (if _returnvalue_2 :!label _label
              (`Widget.RemoveFromParent` _interact_widget)
              (set `self.Can_Interact` false))))
        (else
          (goto _label))))
    (:`else`)))

(event `EnhancedInput|/Game/Source/Input/Actions/IA_Interact`
  (params (ActionValue :type Boolean) (ElapsedSeconds :type "Float (double-precision)") (TriggeredSeconds :type "Float (double-precision)") (InputAction :type "InputAction Object Reference" :default "/Game/Source/Input/Actions/IA_Interact.IA_Interact"))
  ;[1 0 0] Interact
  (:`Started`
    (if (`self.Can_Interact`)
      (bind (_bblockinghit _binitialoverlap _time _distance _location _impactpoint _normal _impactnormal _physmat _hitactor) (`GameplayStatics.BreakHitResult` (stale `self.ReceiveTick` _outhit)))
      (message `/Game/Source/Blueprints/Interfaces/BI_Interact.InteractLever` _hitactor)
      (message `/Game/Source/Blueprints/Interfaces/BI_Interact.InteractButton` _hitactor self)
      (message `/Game/Source/Blueprints/Interfaces/BI_Interact.InteractLunettes` _hitactor self))))

(event `EnhancedInput|/Game/FirstPerson/Input/Actions/IA_Move`
  (params (ActionValue :type "Vector2D Structure") (ElapsedSeconds :type "Float (double-precision)") (TriggeredSeconds :type "Float (double-precision)") (InputAction :type "InputAction Object Reference" :default "/Game/FirstPerson/Input/Actions/IA_Move.IA_Move"))
  (:`Triggered`
    (`self.AddMovementInput` (`self.GetActorRightVector`) ActionValue_X)
    (`self.AddMovementInput` (`self.GetActorForwardVector`) ActionValue_Y)))

(event `/Game/Source/Blueprints/Interfaces/BI_Damageable.TakeDamage`
  (params (Damage :type "Float (double-precision)"))
  (bind _output_get (set `self.Health` (- (`self.Health`) Damage)))
  (if (<= _output_get 0.0)
    (bind _asbp_fpsplayer_controller (cast `/Game/Source/BP_FPSPlayerController` (`self.GetController`)))
    (`/Game/Source/BP_FPSPlayerController.OnDeath` _asbp_fpsplayer_controller)))

(event `self.ReceiveDestroyed`)

(event `EnhancedInput|/Game/Source/Input/Actions/IA_Look`
  (params (ActionValue :type "Vector2D Structure") (ElapsedSeconds :type "Float (double-precision)") (TriggeredSeconds :type "Float (double-precision)") (InputAction :type "InputAction Object Reference" :default "/Game/Source/Input/Actions/IA_Look.IA_Look"))
  (:`Triggered`
    (`self.AddControllerYawInput` ActionValue_X)
    (`self.AddControllerPitchInput` ActionValue_Y)))

(event `EnhancedInput|/Game/Source/Input/Actions/IA_Jump`
  (params (ActionValue :type Boolean) (ElapsedSeconds :type "Float (double-precision)") (TriggeredSeconds :type "Float (double-precision)") (InputAction :type "InputAction Object Reference" :default "/Game/Source/Input/Actions/IA_Jump.IA_Jump"))
  (:`Started`
    (`self.Jump`))
  (:`Completed`
    (`self.StopJumping`)))

(event `EnhancedInput|/Game/Source/Input/Actions/IA_Run`
  (params (ActionValue :type Boolean) (ElapsedSeconds :type "Float (double-precision)") (TriggeredSeconds :type "Float (double-precision)") (InputAction :type "InputAction Object Reference" :default "/Game/Source/Input/Actions/IA_Run.IA_Run"))
  ;[1 0 0] Si le Character jump, ne pas appliquer le run
  (:`Started`
    (`self.Run`))
  (:`Completed`
    (`self.Stop Run`)))

(event `EnhancedInput|/Game/Source/Input/Actions/IA_Pause`
  (params (ActionValue :type Boolean) (ElapsedSeconds :type "Float (double-precision)") (TriggeredSeconds :type "Float (double-precision)") (InputAction :type "InputAction Object Reference" :default "/Game/Source/Input/Actions/IA_Pause.IA_Pause"))
  (:`Started`
    (bind _asbp_fpsgame_mode (cast `/Game/Source/BP_FPSGameMode` (`GameplayStatics.GetGameMode`)))
    (`/Game/Source/BP_FPSGameMode.PauseGame` _asbp_fpsgame_mode)))

(fn `Glasses Off`
  (set `self.Glasses_On` true)
  (`WidgetBlueprintLibrary.SetColorVisionDeficiencyType` "NormalVision"))

(fn `Glasses On`
  (set `self.Glasses_On` true)
  (`WidgetBlueprintLibrary.SetColorVisionDeficiencyType` "Tritanope" 10.0))

(fn `Run`
  (bind _maxwalkspeed (`CharacterMovementComponent.MaxWalkSpeed` (`self.CharacterMovement`)))
  (set `self.Temp_Walk_Speed` _maxwalkspeed)
  (set `CharacterMovementComponent.MaxWalkSpeed` (* _maxwalkspeed (`self.Running_Speed_Multiplier`)) (`self.CharacterMovement`)))

(fn `Stop Run`
  (set `CharacterMovementComponent.MaxWalkSpeed` (`self.Temp_Walk_Speed`) (`self.CharacterMovement`)))

(fn `UserConstructionScript`)