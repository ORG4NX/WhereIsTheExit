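; BP_Door is a proximity door that swings open when a Character overlaps it, provided CanBeOpened is true.
; A Door timeline lerps PivotPoint yaw from 0 to 90 degrees, and reverses whenever a Character ends overlap, without checking CanBeOpened.
; A timeline event track plays an opening or closing sound at the Porte component, chosen by playback direction.
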(event `self.ReceiveBeginPlay`
  (set `self.Player` (`GameplayStatics.GetPlayerCharacter` 0)))

(event `self.ReceiveActorBeginOverlap`
  (params (OtherActor :type "Actor Object Reference"))
  (bind _returnvalue (`SceneComponent.K2_GetComponentLocation` (`self.Porte`)))
  (if (`self.Can_be_Opened`)
    (cast `Character` OtherActor)
    (bind (_direction _newtrack_0) (`Timeline|Door` :!label _label)
      (:`Update`
        (`SceneComponent.K2_SetRelativeRotation` (`self.pivot_point`) (`KismetMathLibrary.MakeRotator` 0.0 0.0 (`KismetMathLibrary.Lerp` 0.0 90.0 _newtrack_0)) false false))
      (:`Play_Door_Sound`
        (switch `ETimelineDirection` _direction
          (:`Forward`
            (`GameplayStatics.PlaySoundAtLocation` "/Game/Source/Sound_Effects/Clap_Ouverture_Porte_.Clap_Ouverture_Porte_" _returnvalue (struct) 0.5 1.0 0.0 null null null null))
          (:`Backward`
            (`GameplayStatics.PlaySoundAtLocation` "/Game/Source/Sound_Effects/Clap_fin_porte_.Clap_fin_porte_" _returnvalue (struct) 0.5 1.0 0.0 null null null null)))))))

(event `self.ReceiveActorEndOverlap`
  (params (OtherActor :type "Actor Object Reference"))
  (cast `Character` OtherActor)
  (goto _label :!via `Reverse`))

(fn `UserConstructionScript`)