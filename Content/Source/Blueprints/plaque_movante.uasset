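; Moving platform actor that shuttles a configurable static mesh between its Start and End points once the player pawn enters its trigger box.
; The overlap starts a looping timer and sets the timeline play rate.
; The animation event plays the timeline forward or in reverse by Direction, lerping the platform between world locations cached at BeginPlay and flipping Direction on finish.
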(event `self.ReceiveBeginPlay`
  (set `self.start_ref` (`SceneComponent.K2_GetComponentLocation` (`self.start`)))
  (set `self.end_ref` (`SceneComponent.K2_GetComponentLocation` (`self.end`))))

(event `self.tigger_box.OnComponentBeginOverlap`
  (params (OverlappedComponent :type "PrimitiveComponent Object Reference") (OtherActor :type "Actor Object Reference") (OtherComp :type "PrimitiveComponent Object Reference") (OtherBodyIndex :type Integer) (bFromSweep :type Boolean) (SweepResult :type "HitResult Structure (by ref)"))
  (if (== (`GameplayStatics.GetPlayerPawn` 0) OtherActor)
    (`KismetSystemLibrary.K2_SetTimerDelegate` (`|CreateDelegate` :!event `animation_plateform`) (`self.Timebyevent`) true)
    (`TimelineComponent.SetPlayRate` (`self.animation_platforme`) (`self.playRate`))))

(event `animation_plateform`
  (switch `ETimelineDirection` (`self.Direction`)
    (:`Forward`
      (bind (_direction _newtrack_0) (`Timeline|animation_platforme` :!via `PlayFromStart` :!label _label)
        (:`Update`
          (`SceneComponent.K2_SetWorldLocation` (`self.plateform`) (`KismetMathLibrary.VLerp` (`self.start_ref`) (`self.end_ref`) _newtrack_0) false false))
        (:`Finished`
          (switch `ETimelineDirection` (`self.Direction`)
            (:`Forward`
              (set `self.Direction` "Backward"))
            (:`Backward`
              (set `self.Direction` "Forward"))))))
    (:`Backward`
      (goto _label :!via `ReverseFromEnd`))))

(fn `UserConstructionScript`
  (locals (NewLocalVar :type "StaticMesh Object Reference"))
  (`StaticMeshComponent.SetStaticMesh` (`self.plateform`) (`self.staticmesh`)))