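; BP_FatWall is a wall that moves upward with door sound effects when ActivateWallMovement is called.
; A one-second timer triggers the Move_Wall timeline, whose track blends a per-update Z world offset added to the Locator component, so movement accumulates each tick rather than interpolating between fixed positions.
; Timeline event tracks play the long lifting sound and the reverberant ending sound at the Locator's location.
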(event `/Game/Source/Blueprints/Interfaces/BI_Wall.Activate_Wall_Movement`
  (`KismetSystemLibrary.K2_SetTimerDelegate` (delegate `Move`) 1.0))

(event `Move`
  (bind (_direction _newtrack_0) (`Timeline|Move_Wall`)
    (:`Update`
      (`SceneComponent.K2_AddWorldOffset` (`self.Locator`) (`KismetMathLibrary.MakeVector` 0.0 0.0 (`KismetMathLibrary.Lerp` 0.0 50.0 _newtrack_0)) false false))
    (:`Play Sound Long`
      (`GameplayStatics.PlaySoundAtLocation` "/Game/Source/Sounds/SFX_Leveeporte_V2.SFX_Leveeporte_V2" (`SceneComponent.K2_GetComponentLocation` (`self.Locator`)) (struct) 0.3 1.0 0.0 null null null null))
    (:`Play Sound End`
      (`GameplayStatics.PlaySoundAtLocation` "/Game/Source/Sounds/SFX_FinPorteReverbe.SFX_FinPorteReverbe" (`SceneComponent.K2_GetComponentLocation` (`self.Locator`)) (struct) 0.2 1.0 0.0 null null null null))))

(fn `UserConstructionScript`)