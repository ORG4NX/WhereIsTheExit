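; BP_Porte is a door actor that swings open when a Character overlaps it and closes when one leaves.
; Opening requires the CanBeOpened flag, while end overlap always reverses the Door timeline for a Character.
; The timeline drives a yaw lerp on PivotPoint to rotate the door a quarter turn.
; BeginPlay stores the player character, though the graph never reads it.
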(event `self.ReceiveBeginPlay`
  (set `self.Player` (`GameplayStatics.GetPlayerCharacter` 0)))

(event `self.ReceiveActorBeginOverlap`
  (params (OtherActor :type "Actor Object Reference"))
  (if (`self.Can_be_Opened`)
    (cast `Character` OtherActor)
    (bind (_direction _newtrack_0) (`Timeline|Door` :!label _label)
      (:`Update`
        (`SceneComponent.K2_SetRelativeRotation` (`self.pivot_point`) (`KismetMathLibrary.MakeRotator` 0.0 0.0 (`KismetMathLibrary.Lerp` 0.0 90.0 _newtrack_0)) false false)))))

(event `self.ReceiveActorEndOverlap`
  (params (OtherActor :type "Actor Object Reference"))
  (cast `Character` OtherActor)
  (goto _label :!via `Reverse`))

(fn `UserConstructionScript`)