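; BP_GoodButton is an interactable button that unlocks a door in the level.
; It starts interactable and turns that off on first interaction, so it works only once.
; Interacting plays Press, waits briefly, calls Release, then finds a BP_Door through GetActorOfClass and sets its CanBeOpened flag to true.
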(event `self.ReceiveBeginPlay`
  (set `self.Can Interact ?` true))

(event `/Game/Source/Blueprints/Interfaces/BI_Interact.On Interact`
  (params (InteractingCharacter :type "/Game/Source/Character/BP_Character Object Reference"))
  (set `self.Can Interact ?` false)
  (`self.Press`)
  (`KismetSystemLibrary.Delay` 0.2)
  (`self.Release`)
  (bind _returnvalue (`GameplayStatics.GetActorOfClass` "/Game/Source/Blueprints/BP_Door.BP_Door_C"))
  (set `/Game/Source/Blueprints/BP_Door.Can_be_Opened` true _returnvalue))

(fn `Can Interact`
  (returns (`bCanInteract?` :type Boolean))
  (return (`self.Can Interact ?`)))

(fn `UserConstructionScript`
  (`parent.UserConstructionScript`))