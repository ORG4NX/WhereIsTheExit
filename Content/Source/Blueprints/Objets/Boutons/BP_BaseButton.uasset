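; BP_BaseButton is a base interactable button that plays a short press-and-release action.
; On interact, Press blocks further interaction, sets the pressed state, plays a sound at the button and offsets it along Z by PushDistance.
; After a brief delay, Release resets the button's relative location, flips the pressed and released flags and re-enables interaction.
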(event `self.ReceiveBeginPlay`
  (set `self.Can Interact ?` true)
  (set `self.Released` true))

(event `/Game/Source/Blueprints/Interfaces/BI_Interact.On Interact`
  (params (InteractingCharacter :type "/Game/Source/Character/BP_Character Object Reference"))
  (`self.Press`)
  (`KismetSystemLibrary.Delay` 0.2)
  (`self.Release`))

(fn `Can Interact`
  (returns (`bCanInteract?` :type Boolean))
  (return (`self.Can Interact ?`)))

(fn `Press`
  (set `self.Can Interact ?` false)
  (set `self.Pressed` true)
  (set `self.Released` false)
  (`GameplayStatics.PlaySoundAtLocation` "/Game/Source/Assets/Sounds/SFX_Button.SFX_Button" (`SceneComponent.K2_GetComponentLocation` (`self.Button`)) (struct) 1.0 1.0 0.0 null null null null)
  (`SceneComponent.K2_SetRelativeLocation` (`self.Button`) (`KismetMathLibrary.MakeVector` 0.0 0.0 (`self.Push Distance`)) false false))

(fn `Release`
  (set `self.Released` true)
  (set `self.Pressed` false)
  (`SceneComponent.K2_SetRelativeLocation` (`self.Button`) (0.0 0.0 0.0) false false)
  (set `self.Can Interact ?` true))

(fn `UserConstructionScript`)