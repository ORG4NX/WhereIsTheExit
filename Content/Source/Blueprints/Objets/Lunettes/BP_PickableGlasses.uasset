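; BP_PickableGlasses is an interactable pickup that puts glasses on the character who interacts with it.
; On interact it disables further interaction, calls GlassesOn on that character, removes its mesh and triggers wall movement on the BP_FatWall found by class lookup.
; It destroys itself after a short delay.
; A separate TriggerSound function plays the glasses-on sound at its location.
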(event `self.ReceiveBeginPlay`
  (set `self.CanInteract` true))

(event `/Game/Source/Blueprints/Interfaces/BI_Interact.On Interact`
  (params (InteractingCharacter :type "/Game/Source/Character/BP_Character Object Reference"))
  (set `self.CanInteract` false)
  (`/Game/Source/Character/BP_Character.Glasses On` InteractingCharacter)
  (`ActorComponent.K2_DestroyComponent` (`self.StaticMesh`))
  (bind _returnvalue (`GameplayStatics.GetActorOfClass` "/Game/Source/Blueprints/BP_FatWall.BP_FatWall_C"))
  (message `/Game/Source/Blueprints/Interfaces/BI_Wall.Activate_Wall_Movement` _returnvalue)
  (`KismetSystemLibrary.Delay` 0.2)
  (`self.K2_DestroyActor`))

(fn `Can Interact`
  (returns (`bCanInteract?` :type Boolean))
  (return (`self.CanInteract`)))

(fn `TriggerSound`
  (`GameplayStatics.PlaySoundAtLocation` "/Game/Source/Assets/Sounds/SFX_GlassesOn.SFX_GlassesOn" (`self.K2_GetActorLocation`) (struct) 1.0 1.0 0.0 null null null null))

(fn `UserConstructionScript`)